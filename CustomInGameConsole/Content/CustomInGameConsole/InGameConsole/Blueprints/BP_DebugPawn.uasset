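; Debug pawn for the in-game console's photo mode; its graph handles leaving that mode.
; DeactivatePhotoMode resets global time dilation to normal, has the player controller possess the pawn's Instigator and re-enables player character tick.
; It then restores each widget in DisabledWidgets to its saved visibility from the parallel WidgetsPreviousVisibility array and destroys itself.
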(event `Event DeactivatePhotoMode`
  ;[0 0 0] Event DeactivatePhotoMode
  (`GameplayStatics.SetGlobalTimeDilation` 1.0)
  (`Controller.Possess` (`GameplayStatics.GetPlayerController` 0) (`self.GetInstigator`))
  (`self.SetActorTickEnabled` (`GameplayStatics.GetPlayerCharacter` 0) true)
  (if (!= (`KismetArrayLibrary.Array_Length` (`self.DisabledWidgets`)) 0)
    (for (_array_element _array_index) (`self.DisabledWidgets`)
      (`Widget.SetVisibility` _array_element (`|GetArrayItem` (`self.WidgetsPreviousVisibility`) _array_index))))
  (`self.K2_DestroyActor`))

(fn `UserConstructionScript`)